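; Tracer-style playable character with a charge-based directional Blink, a Recall rewind and capsule-resizing crouch.
; Blink sweeps the actor along the movement-input direction and spends a stack, which a guarded delay loop refills one at a time.
; A looping timer shifts transform and HP into history arrays covering about three seconds.
; Recall restores the oldest transform and highest recorded HP, then starts its cooldown and updates the ability widget.
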(event Custom|blink%20charge
  ;[1 1 1] 점멸 충전
  (if (not (Variables|Default|Getbischagingblink))
    (Variables|Default|Setbischagingblink true)
    (Utilities|FlowControl|Delay 3.0)
    (Math|Integer|IncrementInt (Variables|Default|Getblinkstack)
      (:%20%20
        (Variables|Default|Setbischagingblink false)
        (if (< (Variables|Default|Getblinkstack) 3)
          (CallFunction|BlinkCharge))))))

(event Custom|recall%20cooltime
  (Utilities|FlowControl|Delay 12.0)
  (Variables|Default|Setcanrecall true))

(event EventBeginPlay
  (bind _recall_transform (Variables|Default|Getrecall_transform))
  (Utilities|FlowControl|Sequence
    (:then_0
      (bind _asbgminstance (Utilities|Casting|CastToBGMInstance (Game|GetGameInstance))))
    (:then_1
      (Variables|Default|SetHP 175)
      (for (_ _array_index) _recall_transform
        (Utilities|Array|SetArrayElem _recall_transform _array_index (Transformation|GetActorTransform)))
      (Utilities|Time|SetTimerbyFunctionName 0 "record state" 0.1 true))))

(event Collision|EventActorBeginOverlap
  (params (OtherActor :type Actor%20Object%20Reference)))

(event EventTick
  (params (DeltaSeconds :type Float%20%28single-precision%29)))

(event Input|ActionEvents|InputActionSkill1
  (params (Key :type Key%20Structure :default "None"))
  ;[1 1 1] 점멸
  (:Pressed
    (CallFunction|Calculateblinkdirection)
    (CallFunction|Blink)))

(event Input|ActionEvents|InputActionSkill3
  (params (Key :type Key%20Structure :default "None"))
  ;[1 1 1] 점멸
  (:Pressed
    (CallFunction|Calculateblinkdirection)
    (CallFunction|Blink)))

(event Input|ActionEvents|InputActionSkill2
  (params (Key :type Key%20Structure :default "None"))
  (:Pressed
    (if (Variables|Default|Getcanrecall)
      (Variables|Default|Setcanrecall false)
      (CallFunction|SetRecallTransform)
      (CallFunction|SetRecallHp)
      (CallFunction|RecallCooltime)
      (Default|UseAbility (Variables|/Game/jinwook/WBP/WBP_InGame.WBP_InGame_C|GetWBP_AbilityProgress (Variables|/Game/jinwook/BGMInstance.BGMInstance_C|GetPlayerWidgetWBP (stale EventBeginPlay _asbgminstance)))))))

(event Input|AxisEvents|InputAxismoveforward
  (params (AxisValue :type Float%20%28single-precision%29))
  ;[1 1 1] 점멸
  (Variables|Default|SetFmove%20forward AxisValue))

(event Input|AxisEvents|InputAxismoveright
  (params (AxisValue :type Float%20%28single-precision%29))
  ;[1 1 1] 점멸
  (Variables|Default|SetFmove%20right AxisValue))

(event Input|AxisEvents|InputAxiscrouch
  (params (AxisValue :type Float%20%28single-precision%29))
  (if (== AxisValue 1.0)
    (Components|Capsule|SetCapsuleHalfHeight (Variables|Default|GetCapsuleComponent) 48.0 true)
    (else
      (Components|Capsule|SetCapsuleHalfHeight (Variables|Default|GetCapsuleComponent) 96.0 true))))

(fn ConstructionScript)

(fn Calculateblinkdirection
  (Variables|Default|Setblinkdir (Math|Vector|Normalize (+ (* (Transformation|GetActorForwardVector) (Variables|Default|GetFmove%20forward)) (* (Transformation|GetActorRightVector) (Variables|Default|GetFmove%20right)))))
  (return))

(fn Blink
  (if (> (Variables|Default|Getblinkstack) 0)
    (Transformation|SetActorLocation (+ (* (Variables|Default|Getblinkdir) (Variables|Default|Getblinkdistance)) (Transformation|GetActorLocation)) true false)
    (Math|Integer|DecrementInt (Variables|Default|Getblinkstack)
      (:%20%20
        (CallFunction|BlinkCharge))))
  (return))

(fn RecordState
  (bind _recall_hp (Variables|Default|Getrecall_hp))
  (bind _recall_transform (Variables|Default|Getrecall_transform))
  (bind (_arrayindex _arrayelement) (Utilities|Array|ReverseforEachLoop _recall_transform)
    (:LoopBody
      (if (!= _arrayindex 29)
        (Utilities|Array|SetArrayElem _recall_transform (+ _arrayindex 1) _arrayelement)))
    (:Completed
      (Utilities|Array|SetArrayElem _recall_transform 0 (Transformation|GetActorTransform))
      (bind (_arrayindex_2 _arrayelement_2) (Utilities|Array|ReverseforEachLoop _recall_hp)
        (:LoopBody
          (if (!= _arrayindex_2 29)
            (Utilities|Array|SetArrayElem _recall_hp (+ _arrayindex_2 1) _arrayelement_2)))
        (:Completed
          (Utilities|Array|SetArrayElem _recall_hp 0 (Variables|Default|GetHP)))))))

(fn SetRecallTransform
  (Transformation|SetActorTransform (Utilities|Array|Get(acopy) (Variables|Default|Getrecall_transform) 29)))

(fn SetRecallHp
  (Variables|Default|Setrecall_max_hp (Variables|Default|GetHP))
  (for _array_element (Variables|Default|Getrecall_hp)
    (if (> _array_element (Variables|Default|Getrecall_max_hp))
      (bind _output_get (Variables|Default|Setrecall_max_hp _array_element))
      (Variables|Default|SetHP _output_get))))