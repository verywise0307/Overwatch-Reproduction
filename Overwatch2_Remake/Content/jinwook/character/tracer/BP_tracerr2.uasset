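; First-person Tracer-style player character with rapid-fire gun, charge-based Blink and Recall abilities.
; A timer records transform, HP and camera history; Recall steps back through it, restores the highest recorded HP, then cools down.
; Blink teleports with sweep along movement input and recharges stacks over time.
; Looping fire aims spread projectiles from muzzle to camera-trace target; a second trace only prints enemy hits.
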(event Custom|blink%20charge
  ;[1 1 1] 점멸 충전
  (if (not (Variables|Default|Getbischagingblink))
    (Variables|Default|Setbischagingblink true)
    (Utilities|FlowControl|Delay 3.0)
    (Math|Integer|IncrementInt (Variables|Default|Getblinkstack)
      (:%20%20
        (Variables|Default|Setbischagingblink false)
        (if (< (Variables|Default|Getblinkstack) 3)
          (CallFunction|BlinkCharge))))))

(event Custom|recall%20cooltime
  (Utilities|FlowControl|Delay 12.0)
  (Variables|Default|Setcanrecall true)
  (Variables|Default|Setrecall_index 0))

(event Custom|set%20recall%20transform%20event
  (Transformation|SetActorTransform (Utilities|Array|Get(acopy) (Variables|Default|Getrecall_transform) (Variables|Default|Getrecall_index)))
  (Pawn|SetControlRotation (Pawn|GetController) (Utilities|Array|Get(acopy) (Variables|Default|Getrecall_camera) (Variables|Default|Getrecall_index)))
  (bind _result (Math|Integer|IncrementInt (Variables|Default|Getrecall_index))
    (:%20%20
      (if (< _result 30)
        (Utilities|FlowControl|Delay 0.03)
        (CallFunction|SetRecallTransformEvent)))))

(event EventBeginPlay
  (Utilities|FlowControl|Sequence
    (:then_0
      (bind _asbgminstance (Utilities|Casting|CastToBGMInstance (Game|GetGameInstance))))
    (:then_1
      (bind _returnvalue (UserInterface|CreateWidget "/Game/yena/character/WBP_aimpoint.WBP_aimpoint_C"))
      (UserInterface|Viewport|AddtoViewport _returnvalue 0)
      (Variables|Default|SetMaximum%20firing%20distance 1e+02)
      (Variables|Default|SetHP 175)
      (Variables|Default|Setammo 40)
      (CallFunction|Initrecall))))

(event Collision|EventActorBeginOverlap
  (params (OtherActor :type Actor%20Object%20Reference)))

(event EventTick
  (params (DeltaSeconds :type Float%20%28single-precision%29)))

(event Input|ActionEvents|InputActionSkill1
  (params (Key :type Key%20Structure :default "None"))
  ;[1 1 1] 점멸
  (:Pressed
    (CallFunction|Calculateblinkdirection)
    (CallFunction|Blink)))

(event Input|ActionEvents|InputActionSkill3
  (params (Key :type Key%20Structure :default "None"))
  ;[1 1 1] 점멸
  (:Pressed
    (CallFunction|Calculateblinkdirection)
    (CallFunction|Blink)))

(event Input|ActionEvents|InputActionSkill2
  (params (Key :type Key%20Structure :default "None"))
  (:Pressed
    (if (Variables|Default|Getcanrecall)
      (Variables|Default|Setcanrecall false)
      (CallFunction|SetRecallTransformEvent)
      (CallFunction|SetRecallHp)
      (CallFunction|RecallCooltime)
      (Default|UseAbility (Variables|/Game/jinwook/WBP/WBP_InGame.WBP_InGame_C|GetWBP_AbilityProgress (Variables|/Game/jinwook/BGMInstance.BGMInstance_C|GetPlayerWidgetWBP (stale EventBeginPlay _asbgminstance)))))))

(event Input|ActionEvents|InputActionFire
  (params (Key :type Key%20Structure :default "None"))
  (:Pressed
    (Utilities|Time|SetTimerbyFunctionName 0 "shoot" 0.025 true)
    (Variables|Default|Setisfiring true))
  (:Released
    (Utilities|Time|ClearTimerbyFunctionName 0 "shoot")
    (Variables|Default|Setisfiring false)))

(event Input|AxisEvents|InputAxismoveforward
  (params (AxisValue :type Float%20%28single-precision%29))
  ;[1 1 1] 점멸
  (Variables|Default|SetFmove%20forward AxisValue))

(event Input|AxisEvents|InputAxismoveright
  (params (AxisValue :type Float%20%28single-precision%29))
  ;[1 1 1] 점멸
  (Variables|Default|SetFmove%20right AxisValue))

(event Input|AxisEvents|InputAxiscrouch
  (params (AxisValue :type Float%20%28single-precision%29))
  (if (== AxisValue 1.0)
    (Components|Capsule|SetCapsuleHalfHeight (Variables|Default|GetCapsuleComponent) 48.0 true)
    (else
      (Components|Capsule|SetCapsuleHalfHeight (Variables|Default|GetCapsuleComponent) 96.0 true))))

(fn ConstructionScript
  (|CallParentFunction))

(fn Calculateblinkdirection
  (Variables|Default|Setblinkdir (Math|Vector|Normalize (+ (* (Transformation|GetActorForwardVector) (Variables|Default|GetFmove%20forward)) (* (Transformation|GetActorRightVector) (Variables|Default|GetFmove%20right)))))
  (return))

(fn Blink
  (if (> (Variables|Default|Getblinkstack) 0)
    (Transformation|SetActorLocation (+ (* (Variables|Default|Getblinkdir) (Variables|Default|Getblinkdistance)) (Transformation|GetActorLocation)) true false)
    (Math|Integer|DecrementInt (Variables|Default|Getblinkstack)
      (:%20%20
        (CallFunction|BlinkCharge))))
  (return))

(fn RecordState
  (bind _recall_hp (Variables|Default|Getrecall_hp))
  (bind _recall_transform (Variables|Default|Getrecall_transform))
  (bind _recall_camera (Variables|Default|Getrecall_camera))
  (bind (_arrayindex _arrayelement) (Utilities|Array|ReverseforEachLoop _recall_transform)
    (:LoopBody
      (if (!= _arrayindex 29)
        (Utilities|Array|SetArrayElem _recall_transform (+ _arrayindex 1) _arrayelement)))
    (:Completed
      (Utilities|Array|SetArrayElem _recall_transform 0 (Transformation|GetActorTransform))
      (bind (_arrayindex_2 _arrayelement_2) (Utilities|Array|ReverseforEachLoop _recall_hp)
        (:LoopBody
          (if (!= _arrayindex_2 29)
            (Utilities|Array|SetArrayElem _recall_hp (+ _arrayindex_2 1) _arrayelement_2)))
        (:Completed
          (Utilities|Array|SetArrayElem _recall_hp 0 (Variables|Default|GetHP))
          (bind (_arrayindex_3 _arrayelement_3) (Utilities|Array|ReverseforEachLoop _recall_camera)
            (:LoopBody
              (if (!= _arrayindex_3 29)
                (Utilities|Array|SetArrayElem _recall_camera (+ _arrayindex_3 1) _arrayelement_3)))
            (:Completed
              (Utilities|Array|SetArrayElem _recall_camera 0 (Pawn|GetControlRotation :!class /Script/Engine.Pawn)))))))))

(fn SetRecallTransform
  (params (index :type Integer))
  (Transformation|SetActorTransform (Utilities|Array|Get(acopy) (Variables|Default|Getrecall_transform) index))
  (bind _result (Math|Integer|IncrementInt index)
    (:%20%20
      (if (< _result 30)
        (CallFunction|SetRecallTransform _result)))))

(fn SetRecallHp
  (Variables|Default|Setrecall_max_hp (Variables|Default|GetHP))
  (for _array_element (Variables|Default|Getrecall_hp)
    (if (> _array_element (Variables|Default|Getrecall_max_hp))
      (bind _output_get (Variables|Default|Setrecall_max_hp _array_element))
      (Variables|Default|SetHP _output_get))))

(fn Shoot
  (bind _maximum_firing_distance (Variables|Default|GetMaximum%20firing%20distance))
  (bind _firstpersoncameracomponent (Variables|Default|GetFirstPersonCameraComponent))
  (bind _bullet_point (Variables|Default|Getbullet%20point))
  (bind _returnvalue (Math|Vector|GetForwardVector _firstpersoncameracomponent))
  (bind _returnvalue_2 (Transformation|GetWorldLocation _firstpersoncameracomponent))
  (bind _returnvalue_3 (Transformation|GetWorldLocation _bullet_point))
  (bind _returnvalue_4 (* _maximum_firing_distance 1e+02))
  (bind _returnvalue_5 (* _returnvalue _returnvalue_4))
  (bind _returnvalue_6 (+ _returnvalue_2 _returnvalue_5))
  (bind _outactors (Actor|GetAllActorswithTag "projectile"))
  (bind (_outhit _returnvalue_7) (Collision|LineTraceByChannel _returnvalue_2 _returnvalue_6 "TraceTypeQuery1" false _outactors "None"))
  (Game|SpawnActorfromClass "/Game/yena/character/tracer/BP_tracerProjectile.BP_tracerProjectile_C" (Math|Transform|MakeTransform _returnvalue_3 (CallFunction|GetSprayAngle (Math|Vector|Normalize (- (Math|Vector|SelectVector (.location _outhit) _returnvalue_6 _returnvalue_7) _returnvalue_3)) 3.6)) "AlwaysSpawn" 0 0)
  (bind _outactors_2 (Actor|GetAllActorswithTag "projectile"))
  (bind (_outhit_2 _returnvalue_8) (Collision|LineTraceByChannel _returnvalue_3 (+ _returnvalue_3 (* (CallFunction|GetSprayAngle (Math|Vector|Normalize (- (Math|Vector|SelectVector (.location _outhit) _returnvalue_6 _returnvalue_7) _returnvalue_3)) 3.6) (* (Variables|Default|GetMaximum%20firing%20distance) 1e+02))) "TraceTypeQuery1" false _outactors_2 "None"))
  (if _returnvalue_8
    (if (Actor|ActorHasTag (.hitactor _outhit_2) "enemy")
      (Development|PrintString "enemy"))))

(fn Initrecall
  (bind _recall_camera (Variables|Default|Getrecall_camera))
  (bind _recall_transform (Variables|Default|Getrecall_transform))
  (for (_ _array_index) _recall_transform
    (Utilities|Array|SetArrayElem _recall_transform _array_index (Transformation|GetActorTransform)))
  (for (_ _array_index_2) _recall_camera
    (Utilities|Array|SetArrayElem _recall_camera _array_index_2 (Pawn|GetControlRotation :!class /Script/Engine.Pawn)))
  (Utilities|Time|SetTimerbyFunctionName 0 "record state" 0.1 true))